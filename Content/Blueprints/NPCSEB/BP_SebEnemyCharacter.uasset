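; BP_SebEnemyCharacter is an enemy NPC that alternates between two patrol points and detects players, with all logic running on the server.
; BeginPlay writes the first patrol point to the Blackboard, and overlapping either point switches the stored target to the other.
; PawnSensing writes any seen BP_TopDownCharacter to the player Blackboard key.
; The Blueprint only updates Blackboard data and contains no movement logic.
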(event `self.ReceiveBeginPlay`
  (`/Engine/EditorBlueprintResources/ActorMacros.Switch Has Authority`
    (:`Authority`
      (set `self.SebCurrentPoint` (`self.SebPatrolPoint1`))
      (`BlackboardComponent.SetValueAsObject` (`AIBlueprintHelperLibrary.GetBlackboard` null) (`self.SebPatrolKeyName`) (`self.SebCurrentPoint`) :!label _label))))

(event `self.ReceiveActorBeginOverlap`
  (params (OtherActor :type "Actor Object Reference"))
  (`/Engine/EditorBlueprintResources/ActorMacros.Switch Has Authority`
    (:`Authority`
      (if (== (`self.SebPatrolPoint1`) OtherActor)
        (set `self.SebCurrentPoint` (`self.SebPatrolPoint2`))
        (goto _label)
        (elif (== OtherActor (`self.SebPatrolPoint2`))
          (set `self.SebCurrentPoint` (`self.SebPatrolPoint1`))
          (goto _label))))))

(event `self.PawnSensing.OnSeePawn`
  (params (Pawn :type "Pawn Object Reference"))
  (`/Engine/EditorBlueprintResources/ActorMacros.Switch Has Authority`
    (:`Authority`
      (bind _asbp_top_down_character (cast `/Game/TopDown/Blueprints/BP_TopDownCharacter` Pawn))
      (`BlackboardComponent.SetValueAsObject` (`AIBlueprintHelperLibrary.GetBlackboard` null) (`self.SebPlayerKeyName`) _asbp_top_down_character))))

(fn `UserConstructionScript`)