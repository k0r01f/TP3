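; BP_MovingCoin is a collectible coin that moves back and forth along a Displacement vector during a challenge.
; On Tick, only on the server once the challenge starts, it eases its location in and out from the current start point.
; Speed acts as the seconds per leg, after which the start point advances and Displacement flips sign.
; Collecting the coin runs the parent logic and resets the leg timer.
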(event `self.ReceiveBeginPlay`
  (set `self.InitialLocation` (`self.K2_GetActorLocation`))
  (set `self.ElapsedTime` 0.0))

(event `self.CollectCoin`
  (params (PlayerState :type "PlayerState Object Reference"))
  (`parent.CollectCoin` PlayerState)
  (set `self.ElapsedTime` 0.0))

(event `self.ReceiveTick`
  (params (DeltaSeconds :type "Float (single-precision)"))
  (`parent.ReceiveTick` DeltaSeconds)
  (if (and (`KismetSystemLibrary.IsServer`) (`self.bIsChallengeStarted`))
    (bind _output_get (set `self.ElapsedTime` (+ DeltaSeconds (`self.ElapsedTime`))))
    (if (>= _output_get (`self.Speed`))
      (set `self.InitialLocation` (+ (`self.InitialLocation`) (`self.Displacement`)))
      (set `self.Displacement` (* (`self.Displacement`) -1.0))
      (set `self.ElapsedTime` (- (`self.ElapsedTime`) (`self.Speed`))))
    (`self.K2_SetActorLocation` (+ (`self.InitialLocation`) (`|EaseFunction` "EaseInOut" (/ (`self.ElapsedTime`) (`self.Speed`)) (0.0 0.0 0.0) (`self.Displacement`))))))

(fn `UserConstructionScript`
  (`parent.UserConstructionScript`))