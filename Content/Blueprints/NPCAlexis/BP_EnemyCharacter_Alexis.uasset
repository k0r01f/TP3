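; BP_EnemyCharacter_Alexis is an enemy character that patrols between two points and detects the player, feeding both targets to its AI Blackboard.
; On the server, it starts toward PatrolPoint1 and swaps CurrentPoint whenever it overlaps either patrol point, writing the new target to the patrol key.
; PawnSensing writes any seen BP_TopDownCharacter to the player key, with debug prints; nothing here clears that key.
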(event `self.ReceiveBeginPlay`
  (`/Engine/EditorBlueprintResources/ActorMacros.Switch Has Authority`
    (:`Authority`
      (set `self.CurrentPoint` (`self.PatrolPoint1`))
      (`self.UpdatePatrolPointBB` :!label _label))))

(event `self.ReceiveActorBeginOverlap`
  (params (OtherActor :type "Actor Object Reference"))
  (`/Engine/EditorBlueprintResources/ActorMacros.Switch Has Authority`
    (:`Authority`
      (if (== (`self.PatrolPoint1`) OtherActor)
        (set `self.CurrentPoint` (`self.PatrolPoint2`))
        (goto _label)
        (elif (== OtherActor (`self.PatrolPoint2`))
          (set `self.CurrentPoint` (`self.PatrolPoint1`))
          (goto _label))))))

(event `self.PawnSensing.OnSeePawn`
  (params (Pawn :type "Pawn Object Reference"))
  (bind _playerkeyname (`self.PlayerKeyName`))
  (`/Engine/EditorBlueprintResources/ActorMacros.Switch Has Authority`
    (:`Authority`
      (bind _asbp_top_down_character (cast `/Game/TopDown/Blueprints/BP_TopDownCharacter` Pawn))
      (`KismetSystemLibrary.PrintString` "sense player")
      (`KismetSystemLibrary.PrintString` (`KismetStringLibrary.Conv_NameToString` _playerkeyname))
      (`BlackboardComponent.SetValueAsObject` (`AIBlueprintHelperLibrary.GetBlackboard` null) _playerkeyname _asbp_top_down_character))))

(fn `UserConstructionScript`)