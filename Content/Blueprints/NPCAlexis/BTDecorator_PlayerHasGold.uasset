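; Behavior tree decorator for NPC Alexis that passes only when the targeted player holds at least one coin.
; It reads an actor from a blackboard key, casts it to Character and checks CoinCount on its BP_PlayerState.
; An invalid or non-Character actor fails the condition.
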(fn `PerformConditionCheck`
  (params (OwnerActor :type "Actor Object Reference"))
  (returns (ReturnValue :type Boolean))
  (bind _returnvalue (`BTFunctionLibrary.GetBlackboardValueAsActor` (`self.Key`)))
  (if (`KismetSystemLibrary.IsValid` _returnvalue)
    (bind _ascharacter (cast `Character` _returnvalue)
      (:`then`
        (bind _asbp_player_state (cast `/Game/Blueprints/BP_PlayerState` (`Pawn.PlayerState` _ascharacter)))
        (return (> (`/Game/Blueprints/BP_PlayerState.CoinCount` _asbp_player_state) 0)))
      (:`CastFailed`
        _)))
  (return false))