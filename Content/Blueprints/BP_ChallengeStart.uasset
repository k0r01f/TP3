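; BP_ChallengeStart handles the end of a two-player coin challenge.
; On BeginPlay it binds its ChallengeOver handler to an OnChallengeOver dispatcher.
; The handler compares both local players' BP_PlayerState coin counts, then calls ChallengeOver on each BP_PlayerController.
; Both branches currently pass false to both players, and the incoming IsSuccess value is unused.
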(event `self.ReceiveBeginPlay`
  (add `self.OnChallengeOver` (delegate `Event ChallengeOver`)))

(event `Event ChallengeOver` :!signature `self.OnChallengeOver`
  (params (IsSuccess :type Boolean))
  (bind _asbp_player_state (cast `/Game/Blueprints/BP_PlayerState` (`Controller.PlayerState` (`GameplayStatics.GetPlayerController` 0))))
  (bind _asbp_player_state_2 (cast `/Game/Blueprints/BP_PlayerState` (`Controller.PlayerState` (`GameplayStatics.GetPlayerController` 1))))
  (bind _asbp_player_controller (cast `/Game/Blueprints/BP_PlayerController` (`GameplayStatics.GetPlayerController` 0)))
  (bind _asbp_player_controller_2 (cast `/Game/Blueprints/BP_PlayerController` (`GameplayStatics.GetPlayerController` 1)))
  (if (> (`/Game/Blueprints/BP_PlayerState.CoinCount` _asbp_player_state) (`/Game/Blueprints/BP_PlayerState.CoinCount` _asbp_player_state_2))
    (`/Game/Blueprints/BP_PlayerController.Event ChallengeOver` _asbp_player_controller false)
    (`/Game/Blueprints/BP_PlayerController.Event ChallengeOver` _asbp_player_controller_2 false)
    (else
      (`/Game/Blueprints/BP_PlayerController.Event ChallengeOver` _asbp_player_controller false)
      (`/Game/Blueprints/BP_PlayerController.Event ChallengeOver` _asbp_player_controller_2 false))))

(fn `UserConstructionScript`)